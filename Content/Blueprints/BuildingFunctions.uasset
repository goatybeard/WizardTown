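; BuildingFunctions provides a helper that maps a world location to a section and vertex index in a chunked grid level.
; It reads square, chunk and map sizes from the LevelDatabaseActor, keeping the last one found in the world.
; The location is truncated to grid cells, then integer division picks the section and modulo picks the vertex, both flattened X-major into single indices.
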(fn `Find Vertex Index`
  (params (`World Location` :type "Vector Structure"))
  (returns (`Section Index` :type Integer) (`Vertex Index` :type Integer))
  (locals (`Level Data` :type "/Game/Blueprints/LevelDatabaseActor Object Reference"))
  (bind _chunk_size (`/Game/Blueprints/LevelDatabaseActor.Chunk Size` (`local.Level Data`)))
  (bind (_x _y) (break `IntVector` (make `IntVector` (`KismetMathLibrary.FTrunc` (.x (/ `World Location` (`/Game/Blueprints/LevelDatabaseActor.Square Size` (`local.Level Data`))))) (`KismetMathLibrary.FTrunc` (.y (/ `World Location` (`/Game/Blueprints/LevelDatabaseActor.Square Size` (`local.Level Data`))))) (`KismetMathLibrary.FTrunc` (.z (/ `World Location` (`/Game/Blueprints/LevelDatabaseActor.Square Size` (`local.Level Data`))))))))
  (bind _outactors (`GameplayStatics.GetAllActorsOfClass` null "/Game/Blueprints/LevelDatabaseActor.LevelDatabaseActor_C"))
  (for _array_element _outactors
    (set `local.Level Data` _array_element))
  (return (+ (* (/ _x _chunk_size) (+ (`/Game/Blueprints/LevelDatabaseActor.Map Size` (`local.Level Data`)) 1)) (/ _y _chunk_size)) (+ (* (mod _x _chunk_size) (+ _chunk_size 1)) (mod _y _chunk_size))))