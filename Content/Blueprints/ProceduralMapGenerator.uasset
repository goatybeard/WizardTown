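; Procedural terrain generator that builds a chunked procedural mesh at BeginPlay, assigns biomes and spawns trees.
; Chunk sizing comes from a LevelDatabaseActor, which also stores each section's vertex colours and biomes.
; Seeded permutation tables drive four-octave Perlin noise for vertex height and moisture, with moisture written to vertex colour red.
; A second pass normalises moisture and picks biomes from height and moisture, after rescaling biome ranges to the generated heights.
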(event `self.ReceiveBeginPlay`
  (bind _map_stream (`self.Map Stream`))
  (bind _proceduralmesh (`self.ProceduralMesh`))
  (bind _proceduralmesh_2 (`self.ProceduralMesh`))
  (bind _returnvalue (`KismetMathLibrary.RandomIntegerFromStream` 999 _map_stream))
  (bind _outactors (`GameplayStatics.GetAllActorsOfClass` "/Game/Blueprints/LevelDatabaseActor.LevelDatabaseActor_C"))
  (for _array_element _outactors
    _)
  (set `self.Level Data` _array_element)
  (`self.Buid Map`)
  ;[1 1 1] Set up RNG for map manipulation.
  (`KismetMathLibrary.SetRandomStreamSeed` _map_stream (`self.Map Seed`))
  (bind _output_perm (`self.Construct Permutation Table` _returnvalue))
  (set `self.Elevation Perm` _output_perm)
  (bind _output_perm_2 (`self.Construct Permutation Table` _returnvalue))
  (set `self.Moisture Perm` _output_perm_2)
  ;[1 1 1] Loop to add height and Vertex Color noise to map.
  (for _index (range (`ProceduralMeshComponent.GetNumSections` _proceduralmesh_2))
    (bind _vertices (`KismetProceduralMeshLibrary.GetSectionFromProceduralMesh` _proceduralmesh_2 _index))
    ;;[1 1 1] Add noise to Z height of map.
    (for (_array_element_2 _array_index) _vertices
      (bind _x (.x _array_element_2))
      (bind _y (.y _array_element_2))
      (bind _output_z (`self.Set Height` (`self.Elevation Perm`) _x _y))
      (set `self.Z Max` (`KismetMathLibrary.FMax` (`self.Z Max`) _output_z))
      (set `self.Z Min` (`KismetMathLibrary.FMin` (`self.Z Min`) _output_z))
      (`KismetArrayLibrary.Array_Set` _vertices _array_index (`KismetMathLibrary.MakeVector` _x _y _output_z))
      ;;[1 1 1] Make Noisy Moisture map and add to Vertex Color X.
      (bind _output_moisture (`self.Set Moisture` (`self.Moisture Perm`) _x _y))
      (set `self.Moist Max` (`KismetMathLibrary.FMax` (`self.Moist Max`) _output_moisture))
      (set `self.Moist Min` (`KismetMathLibrary.FMin` (`self.Moist Min`) _output_moisture))
      (`KismetArrayLibrary.Array_Set` (`self.Vertex Colors`) _array_index (make `LinearColor` _output_moisture) true)
      ;;[1 1 1] Fill Vertex Biomes with defaut Water for size.
      (`KismetArrayLibrary.Array_Set` (`self.Vertex Biomes`) _array_index "NewEnumerator0" true))
    (`ProceduralMeshComponent.UpdateMeshSection_LinearColor` :`self` (`self.ProceduralMesh`) :`SectionIndex` _index :`Vertices` _vertices :`VertexColors` (`self.Vertex Colors`))
    (`PrimitiveComponent.SetMaterial` (`self.ProceduralMesh`) _index "/Game/Materials/BiomeMaterial.BiomeMaterial")
    ;;[1 1 1] Add Vertex Colors to Map Data.
    (`KismetArrayLibrary.Array_Set` (`/Game/Blueprints/LevelDatabaseActor.Map Data` (`self.Level Data`)) _index (make `/Game/Blueprints/SectionData` (`self.Vertex Colors`) (`self.Vertex Biomes`)) true))
  (`/Game/Blueprints/BiomeCalcs.Rescale Biome Ranges` (`self.Z Max`) (`self.Z Min`))
  (`/Game/Blueprints/BiomeCalcs.Reset Material Biome Ranges`)
  (for _index_2 (range (`ProceduralMeshComponent.GetNumSections` _proceduralmesh))
    (bind _vertices_2 (`KismetProceduralMeshLibrary.GetSectionFromProceduralMesh` _proceduralmesh _index_2))
    (bind (_vertexcolors _vertexbiomes) (break `/Game/Blueprints/SectionData` (`|GetArrayItem` (`/Game/Blueprints/LevelDatabaseActor.Map Data` (`self.Level Data`)) _index_2)))
    ;[1 1 1] Normalizes Moisture range.
    (for (_array_element_3 _array_index_2) _vertexcolors
      (bind _returnvalue_2 (`KismetMathLibrary.NormalizeToRange` (`.R` (break `LinearColor` _array_element_3)) (`self.Moist Min`) (`self.Moist Max`)))
      (`KismetArrayLibrary.Array_Set` _vertexcolors _array_index_2 (make `LinearColor` _returnvalue_2))
      (bind _biome (`/Game/Blueprints/BiomeCalcs.Find Biome` (.z (`|GetArrayItem` _vertices_2 _array_index_2)) _returnvalue_2))
      (`KismetArrayLibrary.Array_Set` _vertexbiomes _array_index_2 _biome)
      (`ProceduralMeshComponent.UpdateMeshSection_LinearColor` :`self` (`self.ProceduralMesh`) :`SectionIndex` _index_2 :`Vertices` _vertices_2 :`VertexColors` _vertexcolors)))
  (bind _points_out (`/Game/Blueprints/NoiseFunctions.Place Trees and Rocks` _proceduralmesh (`KismetMathLibrary.RandomIntegerFromStream` 999 (`self.Map Stream`))))
  (for _array_element_4 _points_out
    ;[1 1 1] Need to frac and lerp for correct Z!!!
    (bind (_section_index _vertex_index) (`/Game/Blueprints/BuildingFunctions.Find Vertex Index` (`KismetMathLibrary.Conv_Vector2DToVector` _array_element_4)))
    (bind _vertices_3 (`KismetProceduralMeshLibrary.GetSectionFromProceduralMesh` (`self.ProceduralMesh`) _section_index))
    (`|SpawnActorFromClass` "/Game/Tree.Tree_C" (`KismetMathLibrary.Conv_VectorToTransform` (`KismetMathLibrary.Conv_Vector2DToVector` _array_element_4 (.z (`|GetArrayItem` _vertices_3 _vertex_index)))) "Undefined" "OverrideRootScale" null null)))

(fn `Buid Map`
  (locals (`Chunk Count` :type Integer :default -1) (Vertices :type "Array of Vector Structure") (Triangles :type "Array of Integer"))
  (bind _triangles (`local.Triangles`))
  (bind _map_size (`/Game/Blueprints/LevelDatabaseActor.Map Size` (`self.Level Data`)))
  (bind _chunk_size (`/Game/Blueprints/LevelDatabaseActor.Chunk Size` (`self.Level Data`)))
  (bind _square_size (`/Game/Blueprints/LevelDatabaseActor.Square Size` (`self.Level Data`)))
  (bind _chunk_size_2 (`/Game/Blueprints/LevelDatabaseActor.Chunk Size` (`self.Level Data`)))
  (bind _returnvalue (- _chunk_size_2 1))
  (bind _returnvalue_2 (+ _chunk_size_2 1))
  (`ProceduralMeshComponent.ClearMeshSection` (`self.ProceduralMesh`) 0)
  ;[1 1 1] Setup for next Chunk
  (for _index (range (+ _map_size 1))
    (for _index_2 (range (+ _map_size 1))
      (`/Engine/EditorBlueprintResources/StandardMacros.IncrementInt` (`local.Chunk Count`)
        (:`  `
          (`KismetArrayLibrary.Array_Clear` (`local.Vertices`))
          (`KismetArrayLibrary.Array_Clear` (`local.Triangles`))
          ;[1 1 1] Create vertex X and Y
          (for _index_3 (range (* _index _chunk_size) (+ (* (+ _index 1) _chunk_size) 1))
            (for _index_4 (range (* _index_2 _chunk_size) (+ (* (+ _index_2 1) _chunk_size) 1))
              ;[1 1 1] Construct Vertices Array
              (`KismetArrayLibrary.Array_Add` (`local.Vertices`) (`KismetMathLibrary.MakeVector` (`KismetMathLibrary.Conv_IntToDouble` (* _index_3 _square_size)) (`KismetMathLibrary.Conv_IntToDouble` (* _index_4 _square_size))))))
          ;[1 1 1] Create Triangles Array
          (for _index_5 (range (+ _returnvalue 1))
            (for _index_6 (range (+ _returnvalue 1))
              (`|ExecutionSequence`
                (:`then_0`
                  (bind _returnvalue_3 (+ _index_6 (* _index_5 _returnvalue_2)))
                  (`KismetArrayLibrary.Array_Add` _triangles _returnvalue_3))
                (:`then_1`
                  (bind _returnvalue_4 (+ _returnvalue_3 1))
                  (`KismetArrayLibrary.Array_Add` _triangles _returnvalue_4))
                (:`then_2`
                  (bind _returnvalue_5 (+ _index_6 (* (+ _index_5 1) _returnvalue_2)))
                  (`KismetArrayLibrary.Array_Add` _triangles _returnvalue_5))
                (:`then_3`
                  (`KismetArrayLibrary.Array_Add` _triangles _returnvalue_5))
                (:`then_4`
                  (`KismetArrayLibrary.Array_Add` _triangles _returnvalue_4))
                (:`then_5`
                  (`KismetArrayLibrary.Array_Add` _triangles (+ _returnvalue_5 1))))))
          (`ProceduralMeshComponent.CreateMeshSection_LinearColor` :`self` (`self.ProceduralMesh`) :`SectionIndex` (`local.Chunk Count`) :`Vertices` (`local.Vertices`) :`Triangles` (`local.Triangles`) :`bCreateCollision` true))))))

(fn `Construct Permutation Table`
  (params (`Input Seed` :type Integer))
  (returns (`Output Perm` :type "Array of Integer"))
  (locals (`Temp Perm` :type "Set of Integer") (`Temp Stream` :type "RandomStream Structure") (`Temp Array` :type "Array of Integer"))
  (bind _temp_perm (`local.Temp Perm`))
  ;[1 1 1] Construct Permutation Table
  (`KismetMathLibrary.SetRandomStreamSeed` (`local.Temp Stream`) `Input Seed`)
  (while (< (`BlueprintSetLibrary.Set_Length` _temp_perm) 256)
    (`BlueprintSetLibrary.Set_Add` _temp_perm (`KismetMathLibrary.RandomIntegerInRangeFromStream` 0 255 (`local.Temp Stream`))))
  (bind _result (`BlueprintSetLibrary.Set_ToArray` _temp_perm))
  (for _index (range 256)
    (`KismetArrayLibrary.Array_Add` _result (`|GetArrayItem` _result _index)))
  (return _result))

(fn `Set Height`
  (params (`Input Perm` :type "Array of Integer") (`Input X` :type "Float (double-precision)") (`Input Y` :type "Float (double-precision)"))
  (returns (`Output Z` :type "Float (double-precision)"))
  (locals (`Temp Z` :type "Float (double-precision)"))
  (bind _returnvalue (* (`/Game/Blueprints/LevelDatabaseActor.Square Size` (`self.Level Data`)) 50.0))
  ;[1 1 1] Set Z with noise
  (set `local.Temp Z` 0.0)
  (for _index (range 4)
    (bind _returnvalue_2 (`KismetMathLibrary.MultiplyMultiply_FloatFloat` 2.0 (`KismetMathLibrary.Conv_IntToDouble` _index)))
    (bind _output_noise (`/Game/Blueprints/NoiseFunctions.Perlin Noise` `Input Perm` (`KismetMathLibrary.MultiplyByPi` (* _returnvalue_2 (- (/ `Input X` _returnvalue) 0.5))) (`KismetMathLibrary.MultiplyByPi` (* _returnvalue_2 (- (/ `Input Y` _returnvalue) 0.5)))))
    (bind _output_get (set `local.Temp Z` (+ (/ _output_noise _returnvalue_2) (`local.Temp Z`)))))
  (return (* (`KismetMathLibrary.MultiplyMultiply_FloatFloat` _output_get (`self.Z Exp`)) (* 1000 (`self.Z Scale`)))))

(fn `Set Moisture`
  (params (`Input Perm` :type "Array of Integer") (`Input X` :type "Float (double-precision)") (`Input Y` :type "Float (double-precision)"))
  (returns (`Output Moisture` :type "Float (double-precision)"))
  (locals (`Temp Moistness` :type "Float (double-precision)"))
  (bind _returnvalue (* (`/Game/Blueprints/LevelDatabaseActor.Square Size` (`self.Level Data`)) 50.0))
  ;[1 1 1] Set Moisture (Vertex Color R) with noise
  (set `local.Temp Moistness` 0.0)
  (for _index (range 4)
    (bind _returnvalue_2 (`KismetMathLibrary.MultiplyMultiply_FloatFloat` 2.0 (`KismetMathLibrary.Conv_IntToDouble` _index)))
    (bind _output_noise (`/Game/Blueprints/NoiseFunctions.Perlin Noise` `Input Perm` (`KismetMathLibrary.MultiplyByPi` (* _returnvalue_2 (- (/ `Input X` _returnvalue) 0.5))) (`KismetMathLibrary.MultiplyByPi` (* _returnvalue_2 (- (/ `Input Y` _returnvalue) 0.5)))))
    (bind _output_get (set `local.Temp Moistness` (+ (/ _output_noise _returnvalue_2) (`local.Temp Moistness`)))))
  (return (+ (/ _output_get 2.0) 0.6)))

(fn `UserConstructionScript`)