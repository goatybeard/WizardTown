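; BiomeCalcs is a helper Blueprint for biome classification on a procedural map, using thresholds stored in the LevelDatabaseActor.
; FindBiome picks one of six biomes from height and moisture through nested threshold checks.
; RescaleBiomeRanges remaps default -1..1 height thresholds to the given height range, keeping moisture values.
; ResetMaterialBiomeRanges copies thresholds into the MapParameters material collection, while BalanceBiomeRatios is an unfinished stub.
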(fn `Balance Biome Ratios`
  (params (`Procedural Map In` :type "ProceduralMeshComponent Object Reference")))

(fn `Find Biome`
  (params (`In Height` :type "Float (double-precision)") (`In Moisture` :type "Float (double-precision)"))
  (returns (Biome :type "/Game/Blueprints/Biomes Enum"))
  (bind _outactors (`GameplayStatics.GetAllActorsOfClass` null "/Game/Blueprints/LevelDatabaseActor.LevelDatabaseActor_C"))
  (for _array_element _outactors
    (bind (_water _beach _plains _forest _rocky _snow) (break `/Game/Blueprints/BiomeRanges` (`/Game/Blueprints/LevelDatabaseActor.Biome Ranges` _array_element)))
    (if (>= `In Height` (`KismetMathLibrary.BreakVector2D` _beach))
      (if (>= `In Height` (`KismetMathLibrary.BreakVector2D` _plains))
        (if (>= `In Moisture` (`.Y` (`KismetMathLibrary.BreakVector2D` _forest)))
          (if (>= `In Height` (`KismetMathLibrary.BreakVector2D` _snow))
            (return "NewEnumerator5")
            (else
              (return "NewEnumerator3")))
          (elif (>= `In Height` (`KismetMathLibrary.BreakVector2D` _rocky))
            (return "NewEnumerator4")
            (else
              (return "NewEnumerator2"))))
        (else
          (return "NewEnumerator1")))
      (else
        (return "NewEnumerator0")))))

(fn `Rescale Biome Ranges`
  (params (`Height Max` :type "Float (double-precision)") (`Height Min` :type "Float (double-precision)"))
  (bind (_water _beach _plains _forest _rocky _snow) (break `/Game/Blueprints/BiomeRanges` (make `/Game/Blueprints/BiomeRanges` (-1.0 0.0))))
  (bind (_x _y) (`KismetMathLibrary.BreakVector2D` _water))
  (bind (_x_2 _y_2) (`KismetMathLibrary.BreakVector2D` _beach))
  (bind (_x_3 _y_3) (`KismetMathLibrary.BreakVector2D` _plains))
  (bind (_x_4 _y_4) (`KismetMathLibrary.BreakVector2D` _forest))
  (bind (_x_5 _y_5) (`KismetMathLibrary.BreakVector2D` _rocky))
  (bind (_x_6 _y_6) (`KismetMathLibrary.BreakVector2D` _snow))
  (bind _outactors (`GameplayStatics.GetAllActorsOfClass` null "/Game/Blueprints/LevelDatabaseActor.LevelDatabaseActor_C"))
  (for _array_element _outactors
    (set `/Game/Blueprints/LevelDatabaseActor.Biome Ranges` (make `/Game/Blueprints/BiomeRanges` (`KismetMathLibrary.MakeVector2D` (`KismetMathLibrary.MapRangeClamped` _x 1.0 -1.0 `Height Max` `Height Min`) _y) (`KismetMathLibrary.MakeVector2D` (`KismetMathLibrary.MapRangeClamped` _x_2 1.0 -1.0 `Height Max` `Height Min`) _y_2) (`KismetMathLibrary.MakeVector2D` (`KismetMathLibrary.MapRangeClamped` _x_3 1.0 -1.0 `Height Max` `Height Min`) _y_3) (`KismetMathLibrary.MakeVector2D` (`KismetMathLibrary.MapRangeClamped` _x_4 1.0 -1.0 `Height Max` `Height Min`) _y_4) (`KismetMathLibrary.MakeVector2D` (`KismetMathLibrary.MapRangeClamped` _x_5 1.0 -1.0 `Height Max` `Height Min`) _y_5) (`KismetMathLibrary.MakeVector2D` (`KismetMathLibrary.MapRangeClamped` _x_6 1.0 -1.0 `Height Max` `Height Min`) _y_6)) _array_element)))

(fn `Reset Material Biome Ranges`
  (bind _outactors (`GameplayStatics.GetAllActorsOfClass` null "/Game/Blueprints/LevelDatabaseActor.LevelDatabaseActor_C"))
  (for _array_element _outactors
    (bind (_water _beach _plains _forest _rocky _snow) (break `/Game/Blueprints/BiomeRanges` (`/Game/Blueprints/LevelDatabaseActor.Biome Ranges` _array_element)))
    (`KismetMaterialLibrary.SetScalarParameterValue` null "/Game/Materials/MapParameters.MapParameters" "Beach Min Height" (`KismetMathLibrary.BreakVector2D` _beach))
    (`KismetMaterialLibrary.SetScalarParameterValue` null "/Game/Materials/MapParameters.MapParameters" "Plains Min Height" (`KismetMathLibrary.BreakVector2D` _plains))
    (`KismetMaterialLibrary.SetScalarParameterValue` null "/Game/Materials/MapParameters.MapParameters" "Forest Min Moist" (`.Y` (`KismetMathLibrary.BreakVector2D` _forest)))
    (`KismetMaterialLibrary.SetScalarParameterValue` null "/Game/Materials/MapParameters.MapParameters" "Rocky Min Height" (`KismetMathLibrary.BreakVector2D` _rocky))
    (`KismetMaterialLibrary.SetScalarParameterValue` null "/Game/Materials/MapParameters.MapParameters" "Snowy Min Height" (`KismetMathLibrary.BreakVector2D` _snow))))